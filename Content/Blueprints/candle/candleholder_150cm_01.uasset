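; Interactable 150cm candleholder actor that toggles its candle flame and light on a single interaction.
; Cursor hover toggles custom depth rendering on the candle mesh.
; Lighting activates the flame particle and ramps light brightness through a timeline, while extinguishing cuts both immediately.
; The lit state flips only when the timeline finishes on lighting, but at once on extinguishing.
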(event `self.ReceiveActorBeginCursorOver`
  ;[1 1 1] Comment
  (`PrimitiveComponent.SetRenderCustomDepth` (`self.CandleMEsh`) true))

(event `self.ReceiveActorEndCursorOver`
  ;[1 1 1] Comment
  (`PrimitiveComponent.SetRenderCustomDepth` (`self.CandleMEsh`) false))

(event `self.OnInteractSingle`
  (bind _lighted (`self.lighted`))
  (bind _candlelight (`self.CandleLight`))
  (bind _candleparticle (`self.CandleParticle`))
  (if _lighted
    (`ActorComponent.Deactivate` _candleparticle)
    (`LightComponent.SetBrightness` _candlelight 0.0)
    (set `self.lighted` (not _lighted) :!label _label)
    (else
      (`ActorComponent.Activate` _candleparticle false)
      (bind (_direction _light) (`Timeline|Timeline_0` :!via `PlayFromStart`)
        (:`Update`
          (`LightComponent.SetBrightness` _candlelight (* _light 5000.0)))
        (:`Finished`
          (goto _label))))))

(fn `UserConstructionScript`)